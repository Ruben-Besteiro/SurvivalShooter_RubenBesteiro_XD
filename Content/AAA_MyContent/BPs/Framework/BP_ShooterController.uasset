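; BP_ShooterController is the shooter's controller that pushes player stats to the HUD.
; Its events for health, ammo and kills each cast HealthBarWidget to WBP_HealthBar and write straight into its widgets.
; Health sets the progress bar percent from the unscaled input, while ammo and kills become text with gun and skull emoji.
; BeginPlay and the construction script are empty, so the widget is not created here.
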(event EventBeginPlay)

(event EventUpdateAmmo
  (params (CurrentReserveAmmo :type Integer) (CurrentChargerAmmo :type Integer))
  (Rendering|Components|TextRender|SetText (Variables|/Game/AAA_MyContent/BPs/Widgets/WBP_HealthBar.WBP_HealthBar_C|GetTextBlock_124 (.AsWBP%20Health%20Bar (Utilities|Casting|CastToWBP_HealthBar (Variables|Default|GetHealthBarWidget)))) (Utilities|Text|ToText(String) (Utilities|String|Append (Utilities|String|Append (Utilities|String|ToString(Integer) CurrentReserveAmmo) "🔫") (Utilities|String|ToString(Integer) CurrentChargerAmmo)))))

(event EventUpdateHealth
  (params (CurrentHealth :type Float%20%28single-precision%29))
  (Progress|SetPercent (Variables|/Game/AAA_MyContent/BPs/Widgets/WBP_HealthBar.WBP_HealthBar_C|GetHealthBar (.AsWBP%20Health%20Bar (Utilities|Casting|CastToWBP_HealthBar (Variables|Default|GetHealthBarWidget)))) CurrentHealth))

(event EventUpdateKills
  (params (K :type Integer))
  (Rendering|Components|TextRender|SetText (Variables|/Game/AAA_MyContent/BPs/Widgets/WBP_HealthBar.WBP_HealthBar_C|GetTextBlock_999 (.AsWBP%20Health%20Bar (Utilities|Casting|CastToWBP_HealthBar (Variables|Default|GetHealthBarWidget)))) (Utilities|Text|ToText(String) (Utilities|String|Append "💀" (Utilities|String|ToString(Integer) K)))))

(fn ConstructionScript)